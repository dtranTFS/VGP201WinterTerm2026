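; BP_Gamemode is the game mode for an FPS, owning the match score and countdown timer and showing both in a HUD.
; On BeginPlay it creates WBP_GameMenu, switches input to game-only, hides the cursor, then pushes the initial timer and score.
; Tick runs DecreaseTimer, whose one-second Delay throttles the countdown, with no end condition here.
; UpdateScore adds points and refreshes the widget through the stored menu reference.
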(event EventTick
  (params (DeltaSeconds :type Float%20%28single-precision%29))
  (Utilities|DecreaseTimer))

(event EventBeginPlay
  (Development|PrintString "Spawning BP_Gamemode" true true "(R=0.000000,G=0.660000,B=1.000000,A=1.000000)" 5.0)
  (CallFunction|SpawnGameMenu)
  (CallFunction|UpdateTimer)
  (CallFunction|UpdateScore))

(fn ConstructionScript)

(fn UpdateTimer
  (bind _aswbp_game_menu (Utilities|Casting|CastToWBP_GameMenu (Variables|Default|GetMenu%20Ref)))
  (Default|UpdateTimer _aswbp_game_menu (Variables|Config|GetGameTimer)))

(fn SpawnGameMenu
  (bind _returnvalue (Game|GetPlayerController 0))
  (bind _returnvalue_2 (UserInterface|CreateWidget "/Game/FPS/Blueprints/Game/GUI/WBP_GameMenu.WBP_GameMenu_C"))
  (bind _output_get (Variables|Default|SetMenu%20Ref _returnvalue_2))
  (UserInterface|Viewport|AddtoViewport _output_get 0)
  (Input|SetInputModeGameOnly _returnvalue false)
  (Variables|/Script/Engine.PlayerController|SetbShowMouseCursor _returnvalue false))

(fn UpdateScore
  (params (ScoreToAdd :type Integer))
  (bind _aswbp_game_menu (Utilities|Casting|CastToWBP_GameMenu (Variables|Default|GetMenu%20Ref)))
  (bind _output_get (Variables|Config|SetScore (+ (Variables|Config|GetScore) ScoreToAdd)))
  (Default|UpdateScore _aswbp_game_menu _output_get))