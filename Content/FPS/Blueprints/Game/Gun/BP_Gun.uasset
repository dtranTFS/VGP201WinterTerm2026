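; BP_Gun is a gun Blueprint that appears to serve as a base for weapons in the FPS game.
; An interface shoot event forwards start and end positions to OnGunShoot, which is empty here.
; Getters expose the damage, fire rate and shoot distance variables, while GetMaxBulletDistance returns without a connected value.
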(event EventBeginPlay)

(event Collision|EventActorBeginOverlap
  (params (OtherActor :type Actor%20Object%20Reference)))

(event EventTick
  (params (DeltaSeconds :type Float%20%28single-precision%29)))

(event EventOnInterfaceShoot
  (params (Start%20Position :type Vector :default "0, 0, 0") (End%20Position :type Vector :default "0, 0, 0"))
  (CallFunction|OnGunShoot Start%20Position End%20Position))

(fn ConstructionScript)

(fn OnGunShoot
  (params (Start%20Position :type Vector) (End%20Position :type Vector)))

(fn GetMaxBulletDistance
  (return))

(fn GetDamage
  (return (Variables|GunVar|GetDamage)))

(fn GetFireRate
  (return (Variables|GunVar|GetFireRate)))

(fn GetShootDistance
  (return (Variables|GunVar|GetShootDistance)))