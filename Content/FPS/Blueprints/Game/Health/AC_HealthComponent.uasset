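; Health component that stores an actor's health and provides damage, healing, death-check and normalized health queries.
; On BeginPlay it initializes itself to MaxHealth through Init, which can also set new bounds.
; Every change routes through SetHealth, which clamps between MinHealth and MaxHealth.
; Heal and Damage reject non-positive amounts with a printed warning; IsDead is true once health reaches MinHealth.
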(event EventBeginPlay
  (bind _maxhealth (Variables|Config|GetMaxHealth))
  (CallFunction|Init (Variables|Config|GetMinHealth) _maxhealth _maxhealth))

(fn Heal
  (params (Heal%20Amt :type Float%20%28double-precision%29))
  (if (> Heal%20Amt 0.0)
    (CallFunction|SetHealth (+ (CallFunction|GetHealth) Heal%20Amt))
    (else
      (Development|PrintString "Heal value must be positive! Dummy"))))

(fn GetHealth
  (return (Variables|Core|GetHealth)))

(fn SetHealth
  (params (NewHealth :type Float%20%28double-precision%29))
  (bind _output_get (Variables|Core|SetHealth (CallFunction|ClampHealth NewHealth)))
  (return _output_get))

(fn ClampHealth
  (params (Value :type Float%20%28double-precision%29))
  (return (Math|Float|Clamp(Float) Value (Variables|Config|GetMinHealth) (Variables|Config|GetMaxHealth))))

(fn Damage
  (params (Damage%20Amt :type Float%20%28double-precision%29))
  (if (> Damage%20Amt 0.0)
    (CallFunction|SetHealth (- (CallFunction|GetHealth) Damage%20Amt))
    (else
      (Development|PrintString "Damage value must be positive! Idiot"))))

(fn HealFull
  (CallFunction|Heal (Variables|Config|GetMaxHealth)))

(fn GetNormalizedHealth
  (return (Math|Float|Clamp(Float) (/ (CallFunction|GetHealth) (Variables|Config|GetMaxHealth)))))

(fn IsDead
  (return (<= (CallFunction|GetHealth) (Variables|Config|GetMinHealth))))

(fn Init
  (params (MinHealth :type Float%20%28double-precision%29) (MaxHealth :type Float%20%28double-precision%29) (NewHealth :type Float%20%28double-precision%29))
  (Variables|Config|SetMinHealth MinHealth)
  (Variables|Config|SetMaxHealth MaxHealth)
  (CallFunction|SetHealth NewHealth))