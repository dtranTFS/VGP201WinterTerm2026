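; AI controller for enemies that runs the BT_EnemyAI behavior tree on BeginPlay.
; When Pawn Sensing sees a pawn, it writes a can-see-player flag and the seen pawn as target to the blackboard.
; A retriggerable delay of twice the sensing interval serves as a lost-sight timeout, clearing both flag and target once sightings stop.
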(event OnSeePawn(PawnSensing)
  (params (Pawn :type Pawn%20Object%20Reference))
  (CallFunction|SetCanSeePlayerBlackboard true Pawn)
  (Utilities|FlowControl|RetriggerableDelay (* (Variables|/Script/AIModule.PawnSensingComponent|GetSensingInterval (Variables|Default|GetPawnSensing)) 2.0))
  (CallFunction|SetCanSeePlayerBlackboard false))

(event EventBeginPlay
  (AI|RunBehaviorTree "/Game/FPS/Blueprints/Game/Enemy/EnemyAI/BT_EnemyAI.BT_EnemyAI"))

(fn ConstructionScript)

(fn SetCanSeePlayerBlackboard
  (params (CanSeePlayer :type Boolean) (PlayerTarget :type Object%20Object%20Reference))
  (bind _blackboard (Variables|Default|GetBlackboard))
  (AI|Components|Blackboard|SetValueasBool _blackboard (Variables|Default|GetBBCanSeePlayerName) CanSeePlayer)
  (AI|Components|Blackboard|SetValueasObject _blackboard (Variables|Default|GetBBPlayerTargetName) PlayerTarget))