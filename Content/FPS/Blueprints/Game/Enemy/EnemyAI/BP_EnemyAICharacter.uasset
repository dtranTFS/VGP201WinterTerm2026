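; BP_EnemyAICharacter is an FPS enemy character that takes damage and removes itself when it or the player dies.
; AnyDamage feeds the health component, then either destroys the actor or prints its remaining health.
; On BeginPlay it binds to BP_Player's PlayerDied dispatcher to destroy itself.
; When destroyed, it unbinds all events from that dispatcher, which also clears other listeners' bindings.
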(event Custom|OnPlayerDied
  (Actor|DestroyActor))

(event Game|Damage|EventAnyDamage
  (params (Damage :type Float%20%28single-precision%29) (DamageType :type Damage%20Type%20Object%20Reference) (InstigatedBy :type Controller%20Object%20Reference) (DamageCauser :type Actor%20Object%20Reference))
  (bind _ac_healthcomponent (Variables|Default|GetAC_HealthComponent))
  (Default|Damage _ac_healthcomponent Damage)
  (if (Default|IsDead _ac_healthcomponent)
    (Actor|DestroyActor)
    (else
      (Development|PrintString (Utilities|String|ToString(Float) (Default|GetHealth _ac_healthcomponent))))))

(event EventBeginPlay
  (bind _asbp_player (Utilities|Casting|CastToBP_Player (Game|GetPlayerCharacter 0)))
  (EventDispatchers|BindEventtoPlayerDied _asbp_player (delegate Custom|OnPlayerDied)))

(event EventDestroyed
  (bind _asbp_player (Utilities|Casting|CastToBP_Player (Game|GetPlayerCharacter 0)))
  (EventDispatchers|UnbindallEventsfromPlayerDied _asbp_player))

(fn ConstructionScript)